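; Test NPC character with a health bar, pawn sensing and a cannon auto-attack.
; Seeing the player character sets a blackboard flag; Tick feeds a Gate that fires delayed cannon shots, though its range-based open/close logic is disconnected.
; Health interface calls forward to BPCDamageSystem, whose death event ragdolls the mesh, then destroys the actor.
; Line-of-fire overlaps are empty, and launch/homing-dash logic is unwired leftover.
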(event OnComponentEndOverlap(Line_Of_Fire)
  (params (OverlappedComponent :type Primitive%20Component%20Object%20Reference) (OtherActor :type Actor%20Object%20Reference) (OtherComp :type Primitive%20Component%20Object%20Reference) (OtherBodyIndex :type Integer))
  ;[1 1 1] Auto_Attack_Within_Range
)

(event OnComponentBeginOverlap(Line_Of_Fire)
  (params (OverlappedComponent :type Primitive%20Component%20Object%20Reference) (OtherActor :type Actor%20Object%20Reference) (OtherComp :type Primitive%20Component%20Object%20Reference) (OtherBodyIndex :type Integer) (bFromSweep :type Boolean) (SweepResult :type Hit%20Result%20Structure%20%28by%20ref%29))
  ;[1 1 1] Auto_Attack_Within_Range
)

(event OnSeePawn(DetectionRange)
  (params (Pawn :type Pawn%20Object%20Reference))
  (Utilities|Casting|CastToBP_TopDownCharacter_Debug_Original Pawn)
  (AI|Components|Blackboard|SetValueasBool (AI|GetBlackboard (AI|GetAIController self)) (Utilities|Name|MakeLiteralName "hasSeenPlayer") true))

(event Custom|Death
  (bind _mesh (Variables|Character|GetMesh))
  (Physics|SetSimulatePhysics _mesh true)
  (Collision|SetCollisionEnabled _mesh "QueryAndPhysics")
  (Development|PrintString "Dead")
  (Utilities|Array|Clear (Variables|Actor|GetTags))
  (Utilities|FlowControl|Delay 0.8)
  (Actor|DestroyActor))

(event Custom|Blocked
  (Development|PrintString "Dead"))

(event EventTick
  (params (DeltaSeconds :type Float%20%28single-precision%29))
  ;[1 1 1] Auto_Attack_Within_Range
  (Utilities|FlowControl|Gate true
    (:Exit
      (Utilities|FlowControl|Delay 1.0)
      (bind _returnvalue (Game|SpawnActorfromClass "/Game/AlexandersContent/Projectiles/BP_Shot_Canon.BP_Shot_Canon_C" (Transformation|GetWorldTransform (Variables|Default|GetFires_from)) "Undefined" "MultiplyWithRoot" self 7.5e+02 0.9 5e+01 7.5e+02 false "NewEnumerator4" "NewEnumerator0" 0 0))
      (Audio|PlaySound2D "/Game/StarterContent/Audio/Explosion_Cue.Explosion_Cue" 0.125 2.5 0.0 0 0)
      (Collision|IgnoreActorwhenMoving (Variables|Collision|GetCapsuleComponent) _returnvalue true))))

(event EventBeginPlay
  (bind _returnvalue (UserInterface|CreateWidget "/Game/AlexandersContent/Widgets/W_HealthBar.W_HealthBar_C" 0 self))
  (UserInterface|SetWidget (Variables|Default|GetHealthBar) _returnvalue))

(fn ConstructionScript
  (bind _bpc_damagesystem (Variables|Default|GetBPC_DamageSystem))
  (EventDispatchers|BindEventtoOnDeath _bpc_damagesystem (EventDispatchers|CreateEvent :!event Custom|Death))
  (EventDispatchers|BindEventtoOnBlocked _bpc_damagesystem (EventDispatchers|CreateEvent :!event Custom|Blocked)))

(fn IGetCurrentHealth
  (return (Variables|/Game/AlexandersContent/BPC/BPC_DamageSystem.BPC_DamageSystem_C|GetHealth (Variables|Default|GetBPC_DamageSystem))))

(fn IGetMaxHealth
  (return (Variables|/Game/AlexandersContent/BPC/BPC_DamageSystem.BPC_DamageSystem_C|GetMaxHealth (Variables|Default|GetBPC_DamageSystem))))

(fn IHeal
  (params (Amount :type Float%20%28double-precision%29))
  (bind _newhealth (Default|Heal (Variables|Default|GetBPC_DamageSystem) Amount))
  (return _newhealth))

(fn ITakeDamage
  (params (DamageInfo :type S%20Damage%20Info%20Structure))
  (bind _wasdamage (Default|TakeDamage (Variables|Default|GetBPC_DamageSystem) DamageInfo))
  (return _wasdamage))