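; BPC_CurrencySystem is a component that holds a character's currency balance and puts a currency status widget on screen.
; On BeginPlay it creates W_CurrencyStatus for player controller 0 and adds it to the viewport.
; SetNewBalance applies an amount to add and an amount to subtract to the stored balance and returns the result, with no bounds check or direct widget update.
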(event EventBeginPlay
  (CallFunction|ShowBalanceonWidget))

(event EventTick
  (params (DeltaSeconds :type Float%20%28single-precision%29)))

(fn SetNewBalance
  (params (AmountToADD :type Integer) (AmountToSubtract :type Integer))
  (Variables|Default|SetCharacterCurrencyBalance (+ (Variables|Default|GetCharacterCurrencyBalance) AmountToADD))
  (bind _output_get (Variables|Default|SetCharacterCurrencyBalance (- (Variables|Default|GetCharacterCurrencyBalance) AmountToSubtract)))
  (return _output_get))

(fn ShowBalanceonWidget
  (bind _returnvalue (UserInterface|CreateWidget "/Game/AlexandersContent/Widgets/W_CurrencyStatus.W_CurrencyStatus_C" (Game|GetPlayerController 0)))
  (UserInterface|Viewport|AddtoViewport _returnvalue 0))