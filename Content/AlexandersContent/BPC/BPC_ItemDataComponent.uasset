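; BPC_ItemDataComponent is an actor component that makes its owner a pickup item carrying an item data row and quantity.
; On BeginPlay it sets the owner to replicate.
; When a character interacts, it passes the row name and quantity to that character's inventory system component and destroys the owner if the add succeeds.
; Its look-at function returns an empty string.
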(event EventBeginPlay
  ;[0.1311 0.3183 1] Replicerar handlingen för nätverkshantering
  (Networking|SetReplicates (Components|GetOwner) true))

(event EventIInteractwith
  (params (I_I_PlayerCharacter :type Character%20Object%20Reference) (PlayerCharacterAsActorRef :type Actor%20Object%20Reference) (DebuggCharacterRef :type BP%20Top%20Down%20Character%20Debug%20Original%20Object%20Reference))
  (bind _bpc_inventorysystem (Variables|/Game/AlexandersContent/Characters/BP_TopDownCharacter_Debug_Original.BP_TopDownCharacter_Debug_Original_C|GetBPC_InventorySystem DebuggCharacterRef))
  ;[1 1 1] Hämtar data om "vem" som "använder sig av functionen" och kollar att den har en inventory, för att sedan skicka sitt "itemID" till denna "vem" och sedan förstör sig själv.
  (Utilities|IsValid _bpc_inventorysystem
    (:Is%20Valid
      (bind _success___bpc_is_f_ati_ (Default|AddtoInventory _bpc_inventorysystem (Variables|Default|GetQuantity) (.rowname (Variables|Default|GetItemDataID))))
      (if _success___bpc_is_f_ati_
        (Actor|DestroyActor (Components|GetOwner))))))

(fn ILookat
  (return ""))