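; BP_NPC1 is an NPC character with a health bar and gated Tick-driven cannon fire on a one-second delay.
; BPC_DamageSystem handles health through interface pass-throughs and reports death, blocks and damage responses.
; Death routes through ROS and MC events to ragdoll the mesh with an impact-based impulse, then destroys the actor.
; Line_Of_Fire gate toggling is disconnected, and the damage-response launch is unreachable.
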(event OnComponentBeginOverlap(Line_Of_Fire)
  (params (OverlappedComponent :type Primitive%20Component%20Object%20Reference) (OtherActor :type Actor%20Object%20Reference) (OtherComp :type Primitive%20Component%20Object%20Reference) (OtherBodyIndex :type Integer) (bFromSweep :type Boolean) (SweepResult :type Hit%20Result%20Structure%20%28by%20ref%29))
  ;[1 1 1] Auto_Attack_Within_Range
)

(event OnComponentEndOverlap(Line_Of_Fire)
  (params (OverlappedComponent :type Primitive%20Component%20Object%20Reference) (OtherActor :type Actor%20Object%20Reference) (OtherComp :type Primitive%20Component%20Object%20Reference) (OtherBodyIndex :type Integer))
  ;[1 1 1] Auto_Attack_Within_Range
)

(event Custom|Death
  (CallFunction|ROSDeath))

(event Custom|Blocked
  (Development|PrintString "Dead"))

(event Custom|DamageResponse
  (params (DamageResponse :type E_DamageResponsive%20Enum :default "NewEnumerator0") (DamageType :type E_DamageType%20Enum :default "NewEnumerator4") (NormalImpact :type Vector) (DamageAmount :type Float%20%28double-precision%29))
  (Variables|Default|SetNormalImpact NormalImpact)
  (Variables|Default|SetDamage%20Amount DamageAmount)
  (Development|PrintString (Utilities|String|EnumtoString DamageType))
  (if false
    (if false
      (Character|LaunchCharacter "500.000000,0.000000,500.000000" false false))))

(event Custom|ROS_Death
  (CallFunction|MCDeath))

(event Custom|MC_Death
  (bind _mesh (Variables|Character|GetMesh))
  (bind _normalimpact (Variables|Default|GetNormalImpact))
  (Physics|SetSimulatePhysics _mesh true)
  (Collision|SetCollisionEnabled _mesh "QueryAndPhysics")
  (Collision|SetCollisionProfileName _mesh "Ragdoll" true :!class /Script/Engine.PrimitiveComponent)
  (Development|PrintString "Dead")
  (Utilities|Array|Clear (Variables|Actor|GetTags))
  (Physics|AddImpulse (Variables|Character|GetMesh) (Math|Vector|MakeVector (* 1e+01 (* (.x _normalimpact) -1.5e+03)) (* 1e+01 (* (.y _normalimpact) -1.5e+03)) (* 1e+01 (* (.z _normalimpact) -3e+03))) "None" false)
  (Utilities|FlowControl|Delay 1e+01)
  (Actor|DestroyActor))

(event EventTick
  (params (DeltaSeconds :type Float%20%28single-precision%29))
  ;[1 1 1] Auto_Attack_Within_Range
  (Utilities|FlowControl|Gate true
    (:Exit
      (Utilities|FlowControl|Delay 1.0)
      (bind _returnvalue (Game|SpawnActorfromClass "/Game/AlexandersContent/Projectiles/BP_Shot_Canon.BP_Shot_Canon_C" (Transformation|GetWorldTransform (Variables|Default|GetFires_from)) "Undefined" "MultiplyWithRoot" self 7.5e+02 0.9 5e+01 7.5e+02 false "NewEnumerator4" "NewEnumerator0" 0 0))
      (Audio|PlaySound2D "/Game/StarterContent/Audio/Explosion_Cue.Explosion_Cue" 0.125 2.5 0.0 0 0)
      (Collision|IgnoreActorwhenMoving (Variables|Collision|GetCapsuleComponent) _returnvalue true))))

(event EventBeginPlay
  (bind _returnvalue (UserInterface|CreateWidget "/Game/AlexandersContent/Widgets/W_HealthBar.W_HealthBar_C" 0 self))
  (UserInterface|SetWidget (Variables|Default|GetHealthBar) _returnvalue))

(fn ConstructionScript
  (bind _bpc_damagesystem (Variables|Default|GetBPC_DamageSystem))
  (EventDispatchers|BindEventtoOnDeath _bpc_damagesystem (EventDispatchers|CreateEvent :!event Custom|Death))
  (EventDispatchers|BindEventtoOnBlocked _bpc_damagesystem (EventDispatchers|CreateEvent :!event Custom|Blocked))
  (EventDispatchers|BindEventtoOnDamageRespond _bpc_damagesystem (EventDispatchers|CreateEvent :!event Custom|DamageResponse)))

(fn IGetCurrentHealth
  (return (Variables|/Game/AlexandersContent/BPC/BPC_DamageSystem.BPC_DamageSystem_C|GetHealth (Variables|Default|GetBPC_DamageSystem))))

(fn IGetMaxHealth
  (return (Variables|/Game/AlexandersContent/BPC/BPC_DamageSystem.BPC_DamageSystem_C|GetMaxHealth (Variables|Default|GetBPC_DamageSystem))))

(fn IHeal
  (params (Amount :type Float%20%28double-precision%29))
  (bind _newhealth (Default|Heal (Variables|Default|GetBPC_DamageSystem) Amount))
  (return _newhealth))

(fn ITakeDamage
  (params (DamageInfo :type S%20Damage%20Info%20Structure))
  (bind _wasdamage (Default|TakeDamage (Variables|Default|GetBPC_DamageSystem) DamageInfo))
  (return _wasdamage))