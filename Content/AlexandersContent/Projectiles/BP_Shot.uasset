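; BP_Shot is a configurable projectile that aims at a target found by its WeaponSystem and deals area damage on impact.
; Homing shots launch high, then ramp up homing acceleration by timeline after a delay; others aim above the target by its distance.
; Impact spawns effects and sound, destroys the projectile, and damages nearby pawns through a damage interface, with a debug sphere trace.
; Construction applies speed, gravity, homing and targeting range.
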(event OnComponentHit(Collision_Sphere)
  (params (HitComponent :type Primitive%20Component%20Object%20Reference) (OtherActor :type Actor%20Object%20Reference) (OtherComp :type Primitive%20Component%20Object%20Reference) (NormalImpulse :type Vector :default "0, 0, 0") (Hit :type Hit%20Result%20Structure%20%28by%20ref%29))
  (bind _location (Collision|BreakHitResult Hit))
  (bind _array (Utilities|Array|MakeArray "ObjectTypeQuery3"))
  ;[1 1 1] Event_On_Hit_Collision
  (Default|CallOnProjectileImpact OtherActor Hit)
  (Effects|SpawnEmitteratLocation (Variables|Effects|GetImpact%20Effect) _location)
  (Audio|PlaySoundatLocation (Variables|Sounds|GetSound) _location "0, 0, 0" 1.0 1.0 0.0 0 0 0 0)
  (Actor|DestroyActor)
  (Utilities|FlowControl|Sequence
    (:then_0
      (bind (_outactors _returnvalue) (Collision|SphereOverlapActors _location 1e+02 _array "/Script/Engine.Pawn"))
      (for _array_element _outactors
        (if _returnvalue
          (Class|BPIDamageAble|ITakeDamage(Message) _array_element (Utilities|Struct|MakeS_DamageInfo (Variables|Default|GetDamage_FROM_WEAPON) false false false (Variables|Default|GetDamage_Respond_From_weapon) (Variables|Default|GetDamage_Type_From_weapon))))))
    (:then_1
      (Collision|MultiSphereTraceForObjects _location _location 1e+02 _array false 0 "ForDuration"))))

(event Custom|Rotate_To_Target
  (bind _target (Variables|Target|GetTarget))
  (bind _target_2 (Variables|Target|GetTarget))
  (bind _projectilemovement (Variables|Default|GetProjectileMovement))
  (bind _returnvalue (Transformation|GetActorLocation _target_2))
  (bind _returnvalue_2 (Transformation|GetActorLocation _target))
  ;[1 1 1] Rotate_Projectile_To_Target
  (if (Variables|ProjectileSettings|GetIsProjectileHoming)
    (Variables|/Script/Engine.MovementComponent|SetVelocity _projectilemovement (* (Math|Vector|GetUnitDirection(Vector) (Transformation|GetActorLocation) (Math|Vector|MakeVector (- (.x _returnvalue_2) 5e+02) (- (.y _returnvalue_2) 5e+02) (+ (.z _returnvalue_2) 5e+03))) (Variables|ProjectileSettings|GetSpeed)))
    (Utilities|FlowControl|Delay 3.0)
    (bind _homingattack (Timeline|Timeline PlayFromStart)
      (:Update
        (Variables|/Script/Engine.ProjectileMovementComponent|SetHomingAccelerationMagnitude _projectilemovement (Math|Float|Lerp 0.0 1e+03 _homingattack))))
    (else
      (Variables|/Script/Engine.MovementComponent|SetVelocity (Variables|Default|GetProjectileMovement) (* (Math|Vector|GetUnitDirection(Vector) (Transformation|GetActorLocation) (Math|Vector|MakeVector (.x _returnvalue) (.y _returnvalue) (+ (.z _returnvalue) (Variables|Target|GetProjectile_Distance)))) (Variables|ProjectileSettings|GetSpeed))))))

(event EventBeginPlay
  ;[1 1 1] Define_Target_Ignore_Value_AND_Create_Sound
  (Audio|SpawnSoundAttached "/Game/StarterContent/Audio/Steam01_Cue.Steam01_Cue" (Variables|Default|GetSound_Trail) "None" (Variables|/Script/Engine.SceneComponent|GetRelativeLocation (Variables|Default|GetSound_Trail)) "0, 0, 0" "KeepRelativeOffset" true 0.5 1.0 0.0 "/Game/AlexandersContent/Sounds/Projectile_location_sound.Projectile_location_sound" 0)
  (Collision|IgnoreActorwhenMoving (Variables|Default|GetCollision_Sphere) (Components|GetOwner) true)
  (bind (_doeshelooklikea_bitch _attackthebitch) (Default|TargetingSystem (Variables|Default|GetWeaponSystem) (Variables|ProjectileSettings|GetTargetRange)))
  (if _doeshelooklikea_bitch
    (if (Variables|ProjectileSettings|GetIsProjectileHoming)
      (Variables|/Script/Engine.ProjectileMovementComponent|SetHomingTargetComponent (Variables|Default|GetProjectileMovement) (Actor|GetComponentbyClass _attackthebitch "/Script/Engine.SceneComponent")))
    (bind _output_get (Variables|Target|SetTarget _attackthebitch))
    (Variables|Target|GetTarget
      (:then
        (Variables|Target|SetProjectile_Distance (Transformation|GetDistanceTo _output_get))
        (Development|PrintString (Utilities|String|ToString(Float) (Transformation|GetDistanceTo _output_get)))
        (CallFunction|RotatetoTarget))
      (:else))))

(fn ConstructionScript
  (bind _projectilemovement (Variables|Default|GetProjectileMovement))
  (Variables|/Game/AlexandersContent/BPC/WeaponSystem.WeaponSystem_C|SetTargetingRangeDefault (Variables|Default|GetWeaponSystem) (Variables|ProjectileSettings|GetTargetRange))
  ;[1 1 1] Changeable_Variables_Projectile_Settings
  (Variables|/Script/Engine.ProjectileMovementComponent|SetInitialSpeed _projectilemovement (Variables|ProjectileSettings|GetSpeed))
  (Variables|/Script/Engine.ProjectileMovementComponent|SetMaxSpeed _projectilemovement (Variables|ProjectileSettings|GetSpeed))
  (Variables|/Script/Engine.ProjectileMovementComponent|SetProjectileGravityScale _projectilemovement (Variables|ProjectileSettings|GetGravity))
  (Variables|/Script/Engine.ProjectileMovementComponent|SetbIsHomingProjectile _projectilemovement (Variables|ProjectileSettings|GetIsProjectileHoming)))