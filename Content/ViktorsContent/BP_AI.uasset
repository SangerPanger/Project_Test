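; BP_AI is an AI-controlled actor that detects the player by sight and flags it on its blackboard.
; When its DetectionRange component sees a BP_TopDownCharacter_Debug_Original, it sets the hasSeenPlayer key to true through its AI controller's blackboard.
; Nothing here resets that key, and BeginPlay only clears the Target variable.
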(event OnSeePawn(DetectionRange)
  (params (Pawn :type Pawn%20Object%20Reference))
  (Utilities|Casting|CastToBP_TopDownCharacter_Debug_Original Pawn)
  (AI|Components|Blackboard|SetValueasBool (AI|GetBlackboard (AI|GetAIController self)) (Utilities|Name|MakeLiteralName "hasSeenPlayer") true))

(event Collision|EventActorBeginOverlap
  (params (OtherActor :type Actor%20Object%20Reference)))

(event EventTick
  (params (DeltaSeconds :type Float%20%28single-precision%29)))

(event EventBeginPlay
  (Variables|Default|SetTarget 0))

(fn ConstructionScript)