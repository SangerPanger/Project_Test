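; BP_Enemy_Ranged is a ranged enemy character that exposes attack, patrol route and movement speed functions.
; Attack plays a montage on the mesh and calls OnAttackEnd whether it completes or is interrupted; no projectile or damage logic appears here.
; GetPatrolRoute returns the stored route.
; SetMovementSpeed maps a speed enum to the CharacterMovement walk speed, but always returns zero.
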(event Custom|Attack
  (Animation|Montage|PlayMontage (Variables|Character|GetMesh) "/Game/ViktorsContent/Animations/MontageOne.MontageOne"
    (:OnCompleted
      _)
    (:OnInterrupted
      _))
  (Default|CallOnAttackEnd))

(fn ConstructionScript)

(fn GetPatrolRoute
  (return (Variables|AI|GetPatrolRoute)))

(fn SetMovementSpeed
  (params (Speed :type E_MovementSpeed%20Enum :default "NewEnumerator0"))
  (Variables|/Script/Engine.CharacterMovementComponent|SetMaxWalkSpeed (Variables|Character|GetCharacterMovement) (Utilities|Select :Index Speed :NewEnumerator0 2.5e+02 :NewEnumerator1 3.5e+02 :NewEnumerator2 375.0 :NewEnumerator3 4e+02 :NewEnumerator4 0.0))
  (return 0.0))